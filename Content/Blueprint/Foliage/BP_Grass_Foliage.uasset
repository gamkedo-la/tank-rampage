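; Grass foliage Blueprint that switches its material to match the current rendering material quality level.
; A looping timer started at BeginPlay polls the level every PollInterval instead of reacting to settings changes.
; High quality selects HighQualityMaterial, while Low, Medium and any other level share LowQualityMaterial.
; Each refresh updates material slot 0 only when the desired material differs from the current one.
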(event `self.ReceiveBeginPlay`
  (`KismetSystemLibrary.K2_SetTimer` null "Refresh Active Material" (`self.Poll Interval`) true))

(fn `Get Material By Current Scalability`
  (returns (Material :type "MaterialInterface Object Reference"))
  (switch `int` (`KismetSystemLibrary.GetRenderingMaterialQualityLevel`) ; 0: Low\n1: High\n2: Medium
    (:`Default`
      _)
    (:`0`
      _)
    (:`1`
      (return (`self.High Quality Material`)))
    (:`2`
      _))
  (return (`self.Low Quality Material`)))

(fn `Refresh Active Material`
  (locals (`Desired Material` :type "MaterialInterface Object Reference"))
  (bind _output_get (set `local.Desired Material` (`self.Get Material By Current Scalability`)))
  (if (!= (`self.GetMaterial` 0) _output_get)
    (`self.SetMaterial` 0 (`local.Desired Material`))))