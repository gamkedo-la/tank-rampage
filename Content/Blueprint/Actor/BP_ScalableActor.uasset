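; BP_ScalableActor spawns one of three actor variants based on the player's overall graphics scalability level.
; On BeginPlay it reads the overall scalability level from Game User Settings and compares it to medium and high thresholds to pick a tier.
; The matching low, medium or high actor component then spawns its actor, with high as the fallback.
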(event `self.ReceiveBeginPlay`
  (`DynamicChildActorComponent.SpawnActor` (`self.Get Actor Component By Scalability`)))

(fn `Get Actor Component By Scalability`
  (returns (NewParam :type "DynamicChildActorComponent Object Reference"))
  (switch `int` (`self.Get Actor Scalability`)
    (:`Default`
      _)
    (:`0`
      (return (`self.Low Scalability Actor`)))
    (:`1`
      (return (`self.Medium Scalability Actor`)))
    (:`2`
      _))
  (return (`self.High Scalability Actor`)))

(fn `Get Actor Scalability`
  (returns (Scalability :type Integer))
  (locals (`Current Scalability` :type Integer :default 0))
  (bind _returnvalue (`GameUserSettings.GetGameUserSettings`))
  (bind _output_get (set `local.Current Scalability` (`GameUserSettings.GetOverallScalabilityLevel` _returnvalue)))
  (if (>= _output_get (`self.High Scalability Threshold`))
    (return 2)
    (elif (>= (`local.Current Scalability`) (`self.Medium Scalability Threshold`))
      (return 1)
      (else
        (return 0)))))

(fn `UserConstructionScript`)