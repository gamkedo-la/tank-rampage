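; Base tank pawn Blueprint that provides visual damage feedback by tinting its materials according to health.
; Initialize Damage Materials creates dynamic material instances for every slot of the supplied primitive components and caches each with its original diffuse color.
; Set Damage Tint scales the cached RGB by an ease-in-out multiplier between full-damage and undamaged values, preserving alpha.
; The event graph and construction script are empty, so nothing here calls these functions.
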(fn `Create Dynamic Material Instances For Component`
  (params (Component :type "PrimitiveComponent Object Reference"))
  (returns (ReturnValue :type "Array of MaterialInstanceDynamic Object Reference"))
  (locals (`Material Instances` :type "Array of MaterialInstanceDynamic Object Reference"))
  (for _index (range (`PrimitiveComponent.GetNumMaterials` Component))
    (bind _returnvalue (`PrimitiveComponent.CreateDynamicMaterialInstance` Component _index (`PrimitiveComponent.GetMaterial` Component _index) "None"))
    (`KismetArrayLibrary.Array_Add` (`local.Material Instances`) _returnvalue))
  (return (`local.Material Instances`)))

(fn `Get Damage Color Multiplier`
  (params (`Health Pct` :type "Float (double-precision)"))
  (returns (`Damage Tint Multiplier` :type "Float (double-precision)"))
  (return (`KismetMathLibrary.FInterpEaseInOut` (`self.Full Damage Color Multiplier`) 1.0 `Health Pct` (`self.Damage Tint Interp Exp`))))

(fn `Initialize Damage Materials`
  (params (`Primitive Components` :type "Array of PrimitiveComponent Object Reference"))
  (locals (Component :type "PrimitiveComponent Object Reference"))
  (for _array_element `Primitive Components`
    (bind _output_get (set `local.Component` _array_element))
    (bind _returnvalue (`self.Create Dynamic Material Instances For Component` _output_get))
    (for _array_element_2 _returnvalue
      (bind _returnvalue_2 (`MaterialInstanceDynamic.K2_GetVectorParameterValue` _array_element_2 (`self.Diffuse Color Parameter Name`)))
      (`KismetArrayLibrary.Array_Add` (`self.Damage Tint Materials`) (make `/Game/Blueprint/Tank/BP_Visual_Damage_Info` _array_element_2 _returnvalue_2)))))

(fn `Set Damage Tint`
  (params (`Health Pct` :type "Float (double-precision)"))
  (locals (`Damage Tint Multiplier` :type "Float (double-precision)" :default 0.0))
  (bind _damage_tint_multiplier (`local.Damage Tint Multiplier`))
  (set `local.Damage Tint Multiplier` (`self.Get Damage Color Multiplier` `Health Pct`))
  (for _array_element (`self.Damage Tint Materials`)
    (`MaterialInstanceDynamic.SetVectorParameterValue` (break `/Game/Blueprint/Tank/BP_Visual_Damage_Info` _array_element) (`self.Diffuse Color Parameter Name`) (make `LinearColor` (* (break `LinearColor` (`.OriginalColor_5_6AD1D8BA4E5185F6D8E0E7B14DC42844` (break `/Game/Blueprint/Tank/BP_Visual_Damage_Info` _array_element))) _damage_tint_multiplier) (* (`.G` (break `LinearColor` (`.OriginalColor_5_6AD1D8BA4E5185F6D8E0E7B14DC42844` (break `/Game/Blueprint/Tank/BP_Visual_Damage_Info` _array_element)))) _damage_tint_multiplier) (* (`.B` (break `LinearColor` (`.OriginalColor_5_6AD1D8BA4E5185F6D8E0E7B14DC42844` (break `/Game/Blueprint/Tank/BP_Visual_Damage_Info` _array_element)))) _damage_tint_multiplier) (`.A` (break `LinearColor` (`.OriginalColor_5_6AD1D8BA4E5185F6D8E0E7B14DC42844` (break `/Game/Blueprint/Tank/BP_Visual_Damage_Info` _array_element))))))))

(fn `UserConstructionScript`)