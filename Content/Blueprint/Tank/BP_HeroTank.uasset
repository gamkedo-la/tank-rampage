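; Hero tank Blueprint that adds damage camera shake and animated tread visuals on top of its parent class.
; On BeginPlay it binds to HealthComponent changes and spaces instanced tread meshes evenly along the right-side spline.
; Tick shifts each instance a fixed step per frame, independent of DeltaTime or speed, wrapping at spline length.
; A spline-versus-actor forward dot product flips each piece's right axis; only the right tread is handled.
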(event `self.ReceiveBeginPlay`
  (`parent.ReceiveBeginPlay`)
  (add `HealthComponent.OnHealthChanged` (`self.HealthComponent`) (delegate `Health Changed`))
  (`self.Spawn Track Meshs`))

(event `Health Changed`
  (params (HealthComponent :type "HealthComponent Object Reference") (PreviousHealthValue :type "Float (single-precision)") (PreviousMaxHealthValue :type "Float (single-precision)") (EventInstigator :type "Controller Object Reference") (ChangeCauser :type "Actor Object Reference"))
  (if (< (`HealthComponent.GetHealth` HealthComponent) PreviousHealthValue)
    (`GameplayStatics.PlayWorldCameraShake` "/Game/Blueprint/Player/BP_CameraShake.BP_CameraShake_C" (`SceneComponent.K2_GetComponentLocation` (`self.Camera`)) 0.0 10.0)))

(event `self.ReceiveTick`
  (params (DeltaSeconds :type "Float (single-precision)"))
  (`self.AnimateTankTracks` DeltaSeconds)
  (`parent.ReceiveTick` DeltaSeconds))

(fn `AnimateTankTracks`
  (params (DeltaTime :type "Float (double-precision)"))
  (bind _tanktreadposition (`self.TankTreadPosition`))
  (bind _tanktreadspline_right (`self.TankTreadSpline_Right`))
  (bind _tanktreadlength (`self.TankTreadLength`))
  (for _index (range (`InstancedStaticMeshComponent.GetInstanceCount` (`self.TankTreadMesh_Right`)))
    (bind _returnvalue (mod (+ (+ (`|GetArrayItem` _tanktreadposition _index) -20.0) _tanktreadlength) _tanktreadlength))
    (`KismetArrayLibrary.Array_Set` _tanktreadposition _index _returnvalue)
    (bind _returnvalue_2 (`SplineComponent.GetRotationAtDistanceAlongSpline` _tanktreadspline_right _returnvalue "World"))
    (if (< (`KismetMathLibrary.Dot_VectorVector` (`KismetMathLibrary.GetForwardVector` _returnvalue_2) (`self.GetActorForwardVector`)) 0.0)
      (bind _returnvalue_3 (`SplineComponent.GetLocationAtDistanceAlongSpline` _tanktreadspline_right _returnvalue "World"))
      (bind _returnvalue_4 (`KismetMathLibrary.GetForwardVector` _returnvalue_2))
      (bind _returnvalue_5 (`KismetMathLibrary.GetRightVector` _returnvalue_2))
      (`InstancedStaticMeshComponent.UpdateInstanceTransform` (`self.TankTreadMesh_Right`) _index (`KismetMathLibrary.MakeTransform` _returnvalue_3 (`KismetMathLibrary.MakeRotationFromAxes` _returnvalue_4 _returnvalue_5 (0.0 0.0 1.0))) true true true)
      (else
        (`InstancedStaticMeshComponent.UpdateInstanceTransform` (`self.TankTreadMesh_Right`) _index (`KismetMathLibrary.MakeTransform` _returnvalue_3 (`KismetMathLibrary.MakeRotationFromAxes` _returnvalue_4 (* _returnvalue_5 -1.0) (0.0 0.0 1.0))) true true true)))))

(fn `Spawn Track Meshs`
  (locals (TrackPieceLength :type "Float (double-precision)") (NumberMeshs :type Integer) (DistancePerMesh :type "Float (double-precision)"))
  (bind _tanktreadspline_right (`self.TankTreadSpline_Right`))
  (bind _returnvalue (`SplineComponent.GetSplineLength` (`self.TankTreadSpline_Right`)))
  (bind _output_get (set `local.TrackPieceLength` (* (.x (`.Max` (break `Box` (`StaticMesh.GetBoundingBox` (`StaticMeshComponent.StaticMesh` (`self.TankTreadMesh_Right`)))))) 1.7)))
  (set `self.TankTreadLength` _returnvalue)
  (bind _output_get_2 (set `local.NumberMeshs` (`KismetMathLibrary.FTrunc` (/ _returnvalue _output_get))))
  (set `local.DistancePerMesh` (/ (`SplineComponent.GetSplineLength` (`self.TankTreadSpline_Right`)) _output_get_2))
  (for _index (range (+ _output_get_2 1))
    (bind _returnvalue_2 (* _index (`local.DistancePerMesh`)))
    (`KismetArrayLibrary.Array_Add` (`self.TankTreadPosition`) _returnvalue_2)
    (bind _returnvalue_3 (`SplineComponent.GetRotationAtDistanceAlongSpline` _tanktreadspline_right _returnvalue_2 "World"))
    (if (< (`KismetMathLibrary.Dot_VectorVector` (`KismetMathLibrary.GetForwardVector` _returnvalue_3) (`self.GetActorForwardVector`)) 0.0)
      (bind _returnvalue_4 (`SplineComponent.GetLocationAtDistanceAlongSpline` _tanktreadspline_right _returnvalue_2 "World"))
      (bind _returnvalue_5 (`KismetMathLibrary.GetForwardVector` _returnvalue_3))
      (bind _returnvalue_6 (`KismetMathLibrary.GetRightVector` _returnvalue_3))
      (`InstancedStaticMeshComponent.AddInstance` (`self.TankTreadMesh_Right`) (`KismetMathLibrary.MakeTransform` _returnvalue_4 (`KismetMathLibrary.MakeRotationFromAxes` _returnvalue_5 _returnvalue_6 (0.0 0.0 1.0))) true)
      (else
        (`InstancedStaticMeshComponent.AddInstance` (`self.TankTreadMesh_Right`) (`KismetMathLibrary.MakeTransform` _returnvalue_4 (`KismetMathLibrary.MakeRotationFromAxes` _returnvalue_5 (* _returnvalue_6 -1.0) (0.0 0.0 1.0))) true)))))

(fn `UserConstructionScript`
  (`parent.UserConstructionScript`))