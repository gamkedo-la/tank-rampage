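; Base breakable environment actor that uses a Chaos Geometry Collection, with helpers for fracturing it on impact.
; Helpers filter hitting actors (projectiles, tanks, common dynamic object types), derive impulse from velocity and start a one-time lifespan.
; ApplyForces scales strain and radial force fields by impulse, centring strain on the impulse vector rather than impact location.
; Only the break event is wired here, playing a soft-referenced sound once via blocking load.
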(event `self.GeometryCollectionComponent.OnChaosBreakEvent`
  (params (BreakEvent :type "ChaosBreakEvent Structure (by ref)"))
  (`self.Play Break Sfx` BreakEvent_Location))

(fn `Apply Forces`
  (params (`Normal Impulse` :type "Vector Structure") (`Impact Location` :type "Vector Structure"))
  (locals (`Impulse Magnitude` :type "Float (double-precision)" :default 0.0))
  (bind _returnvalue (`KismetMathLibrary.VSize` `Normal Impulse`))
  (bind _fieldsystem (`self.FieldSystem`))
  (if (> _returnvalue 0.0)
    (bind _output_get (set `local.Impulse Magnitude` _returnvalue))
    (`FieldSystemComponent.ApplyPhysicsField` _fieldsystem true "Field_ExternalClusterStrain" null (`RadialFalloff.SetRadialFalloff` (`self.RadialFalloff`) (* _output_get (`self.Strain Field Base Magnitude`)) 0.8 1.0 0.0 (`self.Radial Falloff Radius`) `Normal Impulse` "Field_FallOff_None"))
    (`FieldSystemComponent.ApplyPhysicsField` _fieldsystem true "Field_LinearForce" (`self.FieldSystemMetaDataFilter`) (`RadialVector.SetRadialVector` (`self.RadialVector`) (* _output_get (`self.Radial Force Base Magnitude`)) `Impact Location`))))

(fn `Calculate Actor Impulse`
  (params (Actor :type "Actor Object Reference"))
  (returns (`Normal Impulse` :type "Vector Structure"))
  (return (* (`self.GetActorForwardVector` Actor) (* (`KismetMathLibrary.VSize` (`self.GetVelocity` Actor)) (`self.Impulse`)))))

(fn `Initialize Lifespan`
  (if (not (`self.Lifespan Set`))
    (`self.SetLifeSpan` (`self.Hit Lifespan`))
    (set `self.Lifespan Set` true)))

(fn `Is Projectile`
  (params (Actor :type "Actor Object Reference"))
  (returns (Relevant :type Boolean))
  (cast `Projectile` Actor)
  (return true))

(fn `Is Relevant Actor`
  (params (Actor :type "Actor Object Reference"))
  (returns (Relevant :type Boolean))
  (locals (`Current Actor` :type "Actor Object Reference"))
  (bind _returnvalue (`self.GetComponentByClass` (`local.Current Actor`) "/Script/Engine.PrimitiveComponent"))
  (set `local.Current Actor` Actor)
  (if (`self.Is Projectile` (`local.Current Actor`))
    (return true)
    (else
      (cast `BaseTankPawn` (`local.Current Actor`)
        (:`then`
          (return true))
        (:`CastFailed`
          (`/Engine/EditorBlueprintResources/StandardMacros.IsValid` _returnvalue
            (:`Is Valid`
              (switch `ECollisionChannel` (`PrimitiveComponent.GetCollisionObjectType` _returnvalue)
                (:`ECC_WorldDynamic`
                  _)
                (:`ECC_Pawn`
                  _)
                (:`ECC_PhysicsBody`
                  _)
                (:`ECC_Destructible`
                  _))
              (return true))))))))

(fn `Play Break Sfx`
  (params (`Break Location` :type "Vector Structure"))
  (bind _breaksfx (`self.BreakSfx`))
  (if (`self.BreakPlayed`)
    _
    (elif (`KismetSystemLibrary.IsValidSoftObjectReference` _breaksfx)
      (bind _returnvalue (`KismetSystemLibrary.LoadAsset_Blocking` _breaksfx))
      (bind _assound_base (cast `SoundBase` _returnvalue))
      (`GameplayStatics.PlaySoundAtLocation` _assound_base `Break Location` (struct) 1.0 1.0 0.0 null null null null)
      (set `self.BreakPlayed` true))))

(fn `UserConstructionScript`)