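; BP_Breakable_FenceBase is a breakable fence built on a Chaos Geometry Collection, asleep from BeginPlay because its physics simulation cannot be switched off.
; Overlap with a relevant actor enables simulation, wakes the body and sets collision to block all channels.
; Projectiles also apply forces at their location, along their forward vector and scaled by speed and Impulse.
; A Chaos break event or projectile hit initializes the actor's lifespan.
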(event `self.ReceiveBeginPlay`
  ;[1 1 1] Cannot set simulate physics to false for GeometyCollection so put to sleep
  (`PrimitiveComponent.PutRigidBodyToSleep` (`self.GeometryCollectionComponent`) "None"))

(event `self.GeometryCollectionComponent.OnChaosBreakEvent`
  (params (BreakEvent :type "ChaosBreakEvent Structure (by ref)"))
  (`self.Initialize Lifespan`))

(event `self.ReceiveActorBeginOverlap`
  (params (OtherActor :type "Actor Object Reference"))
  (bind _geometrycollectioncomponent (`self.GeometryCollectionComponent`))
  (if (`self.Is Relevant Actor` OtherActor)
    (`PrimitiveComponent.SetSimulatePhysics` _geometrycollectioncomponent true)
    (`PrimitiveComponent.WakeRigidBody` _geometrycollectioncomponent "None")
    (`PrimitiveComponent.SetCollisionResponseToAllChannels` (`self.GeometryCollectionComponent`) "ECR_Block")
    (if (`self.Is Projectile` OtherActor)
      (`self.Apply Forces` (* (`self.GetActorForwardVector` OtherActor) (* (`KismetMathLibrary.VSize` (`self.GetVelocity` OtherActor)) (`self.Impulse`))) (`self.K2_GetActorLocation` OtherActor))
      (`self.Initialize Lifespan`))))

(fn `UserConstructionScript`
  (`parent.UserConstructionScript`))