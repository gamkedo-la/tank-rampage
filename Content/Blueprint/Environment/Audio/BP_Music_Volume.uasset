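; Music trigger volume that fades its audio component in when player pawn 0 enters and fades it out on exit.
; BeginPlay disables the volume and its tick if it has no sound or is not enabled, otherwise it starts music for a player already inside.
; Audio play-state changes set an Active flag, which lets Tick pause or resume the music with the game's pause state.
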(event `self.ReceiveBeginPlay`
  (bind _success (`self.Init`))
  (if _success
    (add `AudioComponent.OnAudioPlayStateChanged` (`self.Music`) (delegate `On Audio State Changed`))
    (`self.Check Overlap At Start`)))

(event `On Audio State Changed`
  (params (PlayState :type "EAudioComponentPlayState Enum" :default "Playing"))
  (switch `EAudioComponentPlayState` PlayState
    (:`Playing`
      (set `self.Active` true :!label _label))
    (:`Stopped`
      (set `self.Active` false))
    (:`FadingIn`
      (goto _label))))

(event `self.ReceiveActorBeginOverlap`
  (params (OtherActor :type "Actor Object Reference"))
  (if (`self.Is Player` OtherActor)
    (`self.Start Music`)))

(event `self.ReceiveActorEndOverlap`
  (params (OtherActor :type "Actor Object Reference"))
  (if (`self.Is Player` OtherActor)
    (`self.Fade Out Music`)))

(event `self.ReceiveTick`
  (params (DeltaSeconds :type "Float (single-precision)"))
  (`self.Check For Pause`))

(fn `Check For Pause`
  (if (`self.Active`)
    (if (`GameplayStatics.IsGamePaused`)
      (`self.Pause Music`)
      (else
        (`self.Resume Music`)))))

(fn `Check Overlap At Start`
  (if (`self.IsOverlappingActor` (`GameplayStatics.GetPlayerPawn` 0))
    (`self.Start Music`)))

(fn `Fade Out Music`
  (if (`self.Enabled`)
    (`AudioComponent.FadeOut` (`self.Music`) (`self.Fade Out Time`) 0.0 "Linear")
    (set `self.Is Fading Out` true)))

(fn `Init`
  (returns (Success :type Boolean))
  (if (and (`KismetSystemLibrary.IsValid` (`AudioComponent.Sound` (`self.Music`))) (`self.Enabled`))
    (return true)
    (else
      (`self.SetActorTickEnabled` false)
      (set `self.Enabled` false)
      (return false))))

(fn `Is Player`
  (params (`Overlapped Actor` :type "Actor Object Reference"))
  (returns (ReturnValue :type Boolean))
  (return (== `Overlapped Actor` (`GameplayStatics.GetPlayerPawn` 0))))

(fn `Pause Music`
  (if (`self.Enabled`)
    (`AudioComponent.SetPaused` (`self.Music`) true)))

(fn `Resume Music`
  (if (`self.Enabled`)
    (`AudioComponent.SetPaused` (`self.Music`) false)))

(fn `Start Music`
  (if (`self.Enabled`)
    (if (`AudioComponent.IsPlaying` (`self.Music`))
      (if (`self.Is Fading Out`)
        (`AudioComponent.FadeIn` (`self.Music`) (`self.Fade In Time`) 1.0 0.0 "Linear" :!label _label)
        (set `self.Is Fading Out` false))
      (else
        (goto _label)))))

(fn `Stop Music`
  (if (`self.Enabled`)
    (`AudioComponent.StopDelayed` (`self.Music`) (`self.Stop Delay Time`))))

(fn `UserConstructionScript`)