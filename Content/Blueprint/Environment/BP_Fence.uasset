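; BP_Fence is a fence prop that gets knocked away when another actor overlaps it, then removes itself.
; On overlap, the mesh switches to simulated physics, blocks all channels and takes an impulse along the other actor's forward vector, scaled by its speed.
; A lifespan timer then destroys the fence.
; A TODO marks it for replacement by a Chaos geometry-collection breakable actor.
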(event `self.ReceiveActorBeginOverlap`
  (params (OtherActor :type "Actor Object Reference"))
  (bind _mesh (`self.Mesh`))
  (`PrimitiveComponent.SetSimulatePhysics` _mesh true)
  (`PrimitiveComponent.SetCollisionResponseToAllChannels` (`self.Mesh`) "ECR_Block")
  (`PrimitiveComponent.AddImpulse` _mesh (* (`self.GetActorForwardVector` OtherActor) (* (`KismetMathLibrary.VSize` (`self.GetVelocity` OtherActor)) (`self.Impulse`))) "None" false)
  (`self.SetLifeSpan` (`self.Hit Lifespan`)))

(fn `UserConstructionScript`)