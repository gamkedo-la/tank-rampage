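; BP_InstMeshSpawner is an editor-only environment tool that scatters instances of a static mesh inside an influence box.
; SpawnInstances clears the instanced mesh component, then adds world-space instances from transforms with random yaw and uniform random scale.
; Each random point in the box is line-traced vertically to the ground and offset by the scaled mesh half-height, keeping the raw point if nothing is hit.
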(event `Spawn Instances`
  (`self.Create Instances`))

(fn `Calculate Spawn Transforms`
  (returns (`Output Spawn Transforms` :type "Array of Transform Structure"))
  (locals (`Instance Index` :type Integer) (`Mesh Offset` :type "Float (double-precision)") (`Spawn Transforms` :type "Array of Transform Structure") (Scale :type "Float (double-precision)" :default 0.0))
  (bind (_mesh_scale_range_x _mesh_scale_range_y) (`KismetMathLibrary.BreakVector2D` (`self.Mesh Scale Range`)))
  (set `local.Mesh Offset` (.z (`.BoxExtent` (`KismetMathLibrary.BreakBoxSphereBounds` (`StaticMesh.GetBounds` (`StaticMeshComponent.StaticMesh` (`self.Mesh`)))))))
  (while (< (`local.Instance Index`) (`self.Num Instances`))
    (bind _output_get (set `local.Scale` (`KismetMathLibrary.RandomFloatInRange` _mesh_scale_range_x _mesh_scale_range_y)))
    (bind _spawn_location (`self.Get Spawn Location` (* (`local.Mesh Offset`) _output_get)))
    (`KismetArrayLibrary.Array_Add` (`local.Spawn Transforms`) (`KismetMathLibrary.MakeTransform` _spawn_location (`KismetMathLibrary.MakeRotator` 0.0 0.0 (`KismetMathLibrary.RandomFloatInRange` -180.0 180.0)) (`KismetMathLibrary.Conv_DoubleToVector` (`local.Scale`))))
    (`/Engine/EditorBlueprintResources/StandardMacros.IncrementInt` (`local.Instance Index`)))
  (return (`local.Spawn Transforms`)))

(fn `Create Instances`
  (locals (`Instance Index` :type Integer) (`Mesh Offset` :type "Float (double-precision)") (`Spawn Transforms` :type "Array of Transform Structure"))
  (if (`TRBlueprintFunctionLibrary.IsRunningInEditor` null)
    (`/Engine/EditorBlueprintResources/StandardMacros.IsValid` (`StaticMeshComponent.StaticMesh` (`self.Mesh`))
      (:`Is Valid`
        (`InstancedStaticMeshComponent.ClearInstances` (`self.Mesh`))
        (`|ExecutionSequence`
          (:`then_0`
            (bind _output_spawn_transforms (`self.Calculate Spawn Transforms`))
            (set `local.Spawn Transforms` _output_spawn_transforms))
          (:`then_1`
            (for _array_element (`local.Spawn Transforms`)
              (`InstancedStaticMeshComponent.AddInstance` (`self.Mesh`) _array_element true))))))))

(fn `Get Spawn Location`
  (params (`Mesh Offset` :type "Float (double-precision)"))
  (returns (`Spawn Location` :type "Vector Structure"))
  (locals (`Initial Spawn Location` :type "Vector Structure") (Offset :type "Float (double-precision)"))
  (bind (_origin _boxextent) (`KismetSystemLibrary.GetComponentBounds` (`self.Influence Box`)))
  (set `local.Offset` `Mesh Offset`)
  (bind _output_get (set `local.Initial Spawn Location` (`KismetMathLibrary.RandomPointInBoundingBox` _origin _boxextent)))
  (bind (_outhit _returnvalue) (`KismetSystemLibrary.LineTraceSingle` (+ _output_get (`KismetMathLibrary.MakeVector` 0.0 0.0 (`self.Ground Trace Extent`))) (- _output_get (`KismetMathLibrary.MakeVector` 0.0 0.0 (`self.Ground Trace Extent`))) "TraceTypeQuery1")) ; Clamp to Ground
  (if _returnvalue
    (return (+ (`.Location` (`GameplayStatics.BreakHitResult` _outhit)) (`local.Offset`)))
    (else
      (return (`local.Initial Spawn Location`)))))

(fn `UserConstructionScript`
  (locals (`Instance Index` :type Integer) (`Mesh Offset` :type "Float (double-precision)")))