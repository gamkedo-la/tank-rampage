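; BP_ShieldItem is a shield item whose cooldown and maximum value improve as its level rises.
; On initialization it caches the original cooldown time and max value.
; Level changes from 2 to 5 dispatch to per-level functions that alternately shorten the cooldown and raise the max value.
; Each upgrade is computed from the cached originals rather than the current values, so multipliers do not compound.
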(event `self.OnLevelChanged`
  (params (NewLevel :type Integer) (PreviousLevel :type Integer))
  (switch `int` NewLevel
    (:`2`
      (`self.Apply Level 2 Upgrades`))
    (:`3`
      (`self.Apply Level 3 Upgrades`))
    (:`4`
      (`self.Apply Level 4 Upgrades`))
    (:`5`
      (`self.Apply Level 5 Upgrades`))))

(event `self.BlueprintInitialize`
  (params (ItemConfigData :type "ItemConfigData Structure (by ref)"))
  (set `self.Original Cooldown Time Seconds` (`self.CooldownTimeSeconds`))
  (set `self.Original Max Value` (`self.MaxValue`)))

(fn `Apply Level 2 Upgrades`
  (set `self.CooldownTimeSeconds` (/ (`self.Original Cooldown Time Seconds`) 2.0)))

(fn `Apply Level 3 Upgrades`
  (set `self.MaxValue` (* (`self.Original Max Value`) 2.0)))

(fn `Apply Level 4 Upgrades`
  (set `self.CooldownTimeSeconds` (/ (`self.Original Cooldown Time Seconds`) 3.0)))

(fn `Apply Level 5 Upgrades`
  (set `self.MaxValue` (* (`self.Original Max Value`) 3.0)))