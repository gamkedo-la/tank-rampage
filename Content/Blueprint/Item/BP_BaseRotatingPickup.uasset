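; Base class for rotating world pickups that react when a player pawn overlaps them.
; It registers its collision for overlap on BeginPlay and spins around local yaw each Tick at RotationRate.
; On overlap it calls HandleOnPickup, an empty hook here, then FireConsumedEvent.
; That event notifies the item subsystem of a loot pickup only if the item is loot and marked for destroy.
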(event `self.ReceiveBeginPlay`
  (`self.RegisterOverlapEvent` (`self.Collision`)))

(event `self.ReceiveTick`
  (params (DeltaSeconds :type "Float (single-precision)"))
  (`self.K2_AddActorLocalRotation` (`KismetMathLibrary.MakeRotator` 0.0 0.0 (* DeltaSeconds (`self.Rotation Rate`)))))

(event `self.ReceiveOnOverlap`
  (params (PlayerPawn :type "Pawn Object Reference"))
  (`self.Handle On Pickup` PlayerPawn)
  (`self.Fire Consumed Event` PlayerPawn))

(fn `Fire Consumed Event`
  (params (`Player Pawn` :type "Pawn Object Reference"))
  (bind _returnvalue (subsystem `ItemSubsystem`))
  (if (and (`self.Is Loot`) (`self.IsMarkedForDestroy`))
    (`/Engine/EditorBlueprintResources/StandardMacros.IsValid` _returnvalue
      (:`Is Valid`
        (`ItemSubsystem.OnLootPickedUp` _returnvalue self `Player Pawn`)))))

(fn `Handle On Pickup`
  (params (`Player Pawn` :type "Pawn Object Reference")))

(fn `UserConstructionScript`)