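; Health pickup that restores a fraction of the collecting pawn's maximum health.
; On pickup, it finds the pawn's HealthComponent and heals through ApplyDamage with a negative amount scaled by HealthRestoreFraction.
; It compares health before and after, marking itself for destruction only if health increased, so it is not consumed at full health.
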(fn `Handle On Pickup`
  (params (`Player Pawn` :type "Pawn Object Reference"))
  (locals (`Health Component` :type "HealthComponent Object Reference") (`Previous Health` :type "Float (single-precision)"))
  (bind _returnvalue (`self.GetComponentByClass` `Player Pawn` "/Script/TRTank.HealthComponent"))
  (`/Engine/EditorBlueprintResources/StandardMacros.IsValid` _returnvalue
    (:`Is Valid`
      (bind _output_get (set `local.Health Component` _returnvalue))
      (set `local.Previous Health` (`HealthComponent.GetHealth` _output_get))
      (`GameplayStatics.ApplyDamage` `Player Pawn` (* (`HealthComponent.GetMaxHealth` (`local.Health Component`)) (`self.Health Restore Fraction`) -1.0) (`Pawn.GetController` `Player Pawn`) self)
      (if (> (`HealthComponent.GetHealth` (`local.Health Component`)) (`local.Previous Health`))
        (`self.MarkForDestroy`)))))

(fn `UserConstructionScript`)