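; BP_MaxHealth is a leveled item Blueprint that scales a max health value as its level rises.
; On initialization it finds the owner's HealthComponent and caches its max health as the baseline.
; Level changes from 2 to 5 map to stepped percentage bonuses, reaching double at the top level.
; Each bonus is applied to the cached baseline, so increases do not compound, and sets both CurrentValue and MaxValue.
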(event `self.OnLevelChanged`
  (params (NewLevel :type Integer) (PreviousLevel :type Integer))
  (`self.Do Level Changed` NewLevel))

(event `self.BlueprintInitialize`
  (params (ItemConfigData :type "ItemConfigData Structure (by ref)"))
  (bind _returnvalue (`self.GetOwner`))
  (`/Engine/EditorBlueprintResources/StandardMacros.IsValid` _returnvalue
    (:`Is Valid`
      (bind _output_get (set `self.Health Component` (`Actor.GetComponentByClass` _returnvalue "/Script/TRTank.HealthComponent")))
      (`/Engine/EditorBlueprintResources/StandardMacros.IsValid` _output_get
        (:`Is Valid`
          (set `self.Original Max Value` (`HealthComponent.GetMaxHealth` _output_get)))))))

(fn `Do Level Changed`
  (params (Level :type Integer))
  (switch `int` Level
    (:`2`
      (`self.Set Pct Increase` 25.0))
    (:`3`
      (`self.Set Pct Increase` 50.0))
    (:`4`
      (`self.Set Pct Increase` 75.0))
    (:`5`
      (`self.Set Pct Increase` 100.0))))

(fn `Set Pct Increase`
  (params (Value :type "Float (double-precision)"))
  (bind _output_get (set `self.CurrentValue` (* (+ (/ Value 100.0) 1.0) (`self.Original Max Value`))))
  (set `self.MaxValue` _output_get))