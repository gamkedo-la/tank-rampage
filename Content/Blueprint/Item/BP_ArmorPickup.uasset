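; Armor pickup that refills the armor item carried by the collecting player.
; On pickup it finds the named armor PassiveEffect in the pawn's ItemInventory component.
; It raises the armor's value to a set fraction of its maximum without lowering a higher current value, rather than adding to it.
; The pickup marks itself for destruction only if setting the value succeeds.
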(fn `Get Restore Amount`
  (params (Armor :type "PassiveEffect Object Reference"))
  (returns (ReturnValue :type "Float (double-precision)"))
  (return (`KismetMathLibrary.FMax` (* (`Percentage.GetMaxValue` Armor) (`self.Armor Restore Fraction`)) (`Percentage.GetCurrentValue` Armor))))

(fn `Handle On Pickup`
  (params (`Player Pawn` :type "Pawn Object Reference"))
  (locals (`Armor Item` :type "PassiveEffect Object Reference"))
  (bind _returnvalue (`self.GetComponentByClass` `Player Pawn` "/Script/TRItem.ItemInventory"))
  (bind _armor_item (`local.Armor Item`))
  (`/Engine/EditorBlueprintResources/StandardMacros.IsValid` _returnvalue
    (:`Is Valid`
      (bind _aspassive_effect (cast `PassiveEffect` (`ItemInventory.GetItemByName` _returnvalue (`self.Armor Name`))))
      (bind _output_get (set `local.Armor Item` _aspassive_effect))
      (`/Engine/EditorBlueprintResources/StandardMacros.IsValid` _output_get
        (:`Is Valid`
          (bind _returnvalue_2 (`PassiveEffect.SetCurrentValue` _armor_item (`self.Get Restore Amount` _armor_item)))
          (if _returnvalue_2
            (`self.MarkForDestroy`)))))))

(fn `UserConstructionScript`)