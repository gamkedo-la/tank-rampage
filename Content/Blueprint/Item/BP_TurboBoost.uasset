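; BP_TurboBoost is a leveled item that provides a timed turbo boost through an attribute multiplier.
; On initialization it adds the effect duration to the configured cooldown, which counts from activation, and sets the base boost.
; Level changes up to level 4 call per-level upgrade functions, each passing a larger total percentage that replaces the multiplier rather than stacking.
; This graph only configures values and contains no activation logic.
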(event `self.BlueprintInitialize`
  (params (ItemConfigData :type "ItemConfigData Structure (by ref)"))
  (set `self.CooldownTimeSeconds` (+ ItemConfigData_CooldownTimeSeconds (`self.DurationSeconds`)))
  (`self.Increase Turbo Boost` 50.0))

(event `self.OnLevelChanged`
  (params (NewLevel :type Integer) (PreviousLevel :type Integer))
  (switch `int` NewLevel
    (:`2`
      (`self.Apply Level 2 Upgrades`))
    (:`3`
      (`self.Apply Level 3 Upgrades`))
    (:`4`
      (`self.Apply Level 4 Upgrades`))))

(fn `Apply Level 2 Upgrades`
  (`self.Increase Turbo Boost` 100.0))

(fn `Apply Level 3 Upgrades`
  (`self.Increase Turbo Boost` 150.0))

(fn `Apply Level 4 Upgrades`
  (`self.Increase Turbo Boost` 200.0))

(fn `Increase Turbo Boost`
  (params (`Total Increase Percent` :type "Float (double-precision)"))
  (set `self.AttributeMultiplier` (+ (/ `Total Increase Percent` 100.0) 1.0)))