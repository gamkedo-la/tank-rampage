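; BP_Missiles is a missile weapon Blueprint that sets its firing parameters from item config and weapon level.
; Initialization copies the cooldown time from the item config data.
; Level changes dispatch to per-level upgrade functions: the first upgrade sets launch speed and enables homing, and later ones raise the projectile count.
; The graph only sets variables and contains no firing or spawning logic.
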(event `self.BlueprintInitialize`
  (params (ItemConfigData :type "ItemConfigData Structure (by ref)"))
  (set `self.CooldownTimeSeconds` (`.CooldownTimeSeconds` (break `ItemConfigData` ItemConfigData))))

(event `self.OnLevelChanged`
  (params (NewLevel :type Integer) (PreviousLevel :type Integer))
  (switch `int` NewLevel
    (:`2`
      (`self.Apply Level 2 Upgrades`))
    (:`3`
      (`self.Apply Level 3 Upgrades`))
    (:`4`
      (`self.Apply Level 4 Upgrades`))
    (:`5`
      (`self.Apply Level 5 Upgrades`))))

(fn `Apply Level 2 Upgrades`
  (set `self.ProjectileLaunchSpeed` 5000.0)
  (set `self.bIsHoming` true))

(fn `Apply Level 3 Upgrades`
  (set `self.ProjectileCount` 2))

(fn `Apply Level 4 Upgrades`
  (set `self.ProjectileCount` 3))

(fn `Apply Level 5 Upgrades`
  (set `self.ProjectileCount` 5))