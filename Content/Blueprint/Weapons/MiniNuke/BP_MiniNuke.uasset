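; BP_MiniNuke is the Mini Nuke weapon Blueprint, defining its cooldown, blast radius and level-based upgrades.
; Initialization takes the cooldown from item config data and caches the base inner and outer damage radii.
; Level changes alternate between widening the blast (levels 2 and 4) and shortening the cooldown (levels 3 and 5).
; Radius multipliers apply to the cached base values, while impact impulse grows by a configurable fraction of that increase.
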(event `self.BlueprintInitialize`
  (params (ItemConfigData :type "ItemConfigData Structure (by ref)"))
  (set `self.CooldownTimeSeconds` ItemConfigData_CooldownTimeSeconds)
  (set `self.Initial Damage Inner Radius` (`self.DamageInnerRadius`))
  (set `self.Initial Damage Outer Radius` (`self.DamageOuterRadius`)))

(event `self.OnLevelChanged`
  (params (NewLevel :type Integer) (PreviousLevel :type Integer))
  (switch `int` NewLevel
    (:`2`
      (`self.Apply Level 2 Upgrades`))
    (:`3`
      (`self.Apply Level 3 Upgrades`))
    (:`4`
      (`self.Apply Level 4 Upgrades`))
    (:`5`
      (`self.Apply Level 5 Upgrades`))))

(fn `Apply Level 2 Upgrades`
  (`self.Increase Damage Radius Multiplier` 2.0))

(fn `Apply Level 3 Upgrades`
  (set `self.CooldownTimeSeconds` 60.0))

(fn `Apply Level 4 Upgrades`
  (`self.Increase Damage Radius Multiplier` 3.0))

(fn `Apply Level 5 Upgrades`
  (set `self.CooldownTimeSeconds` 30.0))

(fn `Increase Damage Radius Multiplier`
  (params (Multiplier :type "Float (double-precision)"))
  (set `self.DamageInnerRadius` (* Multiplier (`self.Initial Damage Inner Radius`)))
  (set `self.DamageOuterRadius` (* Multiplier (`self.Initial Damage Outer Radius`)))
  (set `self.ImpactImpulseAmountMultiplier` (`KismetMathLibrary.FMax` (+ (* (- Multiplier 1.0) (`self.Impulse Level Fractional Increase`)) 1.0) 1.0)))