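; BP_MainGun is the main gun weapon, initialized from an item data asset and upgraded as its level changes.
; Initialization copies the cooldown time from the data asset.
; Each level from 2 to 5 calls its own upgrade function, first halving cooldown, then boosting projectile launch speed, then adding a projectile at each of the last two.
; Upgrades modify the current values, so they stack.
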(event `self.BlueprintInitialize`
  (params (InItemDataAsset :type "ItemDataAsset Object Reference"))
  (set `self.CooldownTimeSeconds` (`ItemDataAsset.MainGunCooldownTimeSeconds` InItemDataAsset)))

(event `self.OnLevelChanged`
  (params (NewLevel :type Integer) (PreviousLevel :type Integer))
  (switch `int` NewLevel
    (:`2`
      (`self.Apply Level 2 Upgrades`))
    (:`3`
      (`self.Apply Level 3 Upgrades`))
    (:`4`
      (`self.Apply Level 4 Upgrades`))
    (:`5`
      (`self.Apply Level 5 Upgrades`))))

(fn `Apply Level 2 Upgrades`
  (set `self.CooldownTimeSeconds` (/ (`self.CooldownTimeSeconds`) 2.0)))

(fn `Apply Level 3 Upgrades`
  (set `self.ProjectileLaunchSpeed` (* (`self.ProjectileLaunchSpeed`) 1.5)))

(fn `Apply Level 4 Upgrades`
  (`/Engine/EditorBlueprintResources/StandardMacros.IncrementInt` (`self.ProjectileCount`)))

(fn `Apply Level 5 Upgrades`
  (`/Engine/EditorBlueprintResources/StandardMacros.IncrementInt` (`self.ProjectileCount`)))