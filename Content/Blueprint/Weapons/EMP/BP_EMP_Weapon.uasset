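; Blueprint for the EMP weapon, defining its setup and level-based upgrades.
; On initialization it takes the cooldown from item config data and caches the original influence radius and effect duration.
; Level changes from 2 to 5 alternately enlarge radius and duration, scaling from the cached originals so multipliers do not compound.
; The EMP effect itself is not implemented in these graphs.
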(event `self.OnLevelChanged`
  (params (NewLevel :type Integer) (PreviousLevel :type Integer))
  (switch `int` NewLevel
    (:`2`
      (`self.Apply Level 2 Upgrades`))
    (:`3`
      (`self.Apply Level 3 Upgrades`))
    (:`4`
      (`self.Apply Level 4 Upgrades`))
    (:`5`
      (`self.Apply Level 5 Upgrades`))))

(event `self.BlueprintInitialize`
  (params (ItemConfigData :type "ItemConfigData Structure (by ref)"))
  (set `self.CooldownTimeSeconds` ItemConfigData_CooldownTimeSeconds)
  (set `self.Original Influence Radius` (`self.InfluenceRadius`))
  (set `self.Original Effect Duration` (`self.EffectDuration`)))

(fn `Apply Level 2 Upgrades`
  (set `self.InfluenceRadius` (* (`self.Original Influence Radius`) 2.0)))

(fn `Apply Level 3 Upgrades`
  (set `self.EffectDuration` (* (`self.Original Effect Duration`) 2.0)))

(fn `Apply Level 4 Upgrades`
  (set `self.InfluenceRadius` (* (`self.Original Influence Radius`) 3.0)))

(fn `Apply Level 5 Upgrades`
  (set `self.EffectDuration` (* (`self.Original Effect Duration`) 3.0)))